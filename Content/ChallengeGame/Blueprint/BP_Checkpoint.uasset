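; BP_Checkpoint is a checkpoint actor that moves the player's respawn point when its Box is overlapped, then removes itself.
; The overlap writes the root's world transform, raised slightly in Z, to SpawnTransform on BP_ThirdPersonGameMode, without filtering the overlapping actor.
; A timeline then drives Hue and Time parameters on the Plane's dynamic material as touch feedback, and a short Delay from its Update destroys the actor.
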(event `self.ReceiveBeginPlay`
  ;[1 1 1] Add an animation effect to the touch
  (bind _returnvalue (`KismetMaterialLibrary.CreateDynamicMaterialInstance` "/Game/ChallengeGame/Materials/BaseMaterial/M_Background.M_Background"))
  (`PrimitiveComponent.SetMaterial` (`self.Plane`) 0 _returnvalue))

(event `self.Box.OnComponentBeginOverlap`
  (params (OverlappedComponent :type "PrimitiveComponent Object Reference") (OtherActor :type "Actor Object Reference") (OtherComp :type "PrimitiveComponent Object Reference") (OtherBodyIndex :type Integer) (bFromSweep :type Boolean) (SweepResult :type "HitResult Structure (by ref)"))
  (bind (_transform_location _transform_rotation _transform_scale) (`KismetMathLibrary.BreakTransform` (`self.Transform`)))
  ;[1 1 1] Record the location of the checkpoint, update to the GameMode interior, and when the character regenerates, it will regenerate in the new location.
  (set `self.Transform` (`SceneComponent.K2_GetComponentToWorld` (`self.DefaultSceneRoot`)))
  (set `self.Transform` (`KismetMathLibrary.MakeTransform` (+ _transform_location (0.0 0.0 50.0)) _transform_rotation _transform_scale))
  (bind _asbp_third_person_game_mode (cast `/Game/ChallengeGame/Demo/ThirdPerson/Blueprints/BP_ThirdPersonGameMode` (`GameplayStatics.GetGameMode`)))
  (set `/Game/ChallengeGame/Demo/ThirdPerson/Blueprints/BP_ThirdPersonGameMode.Spawn Transform` (`self.Transform`) _asbp_third_person_game_mode)
  ;[1 1 1] Add an animation effect to the touch
  (bind (_direction `_新建轨道_0`) (`Timeline|Time`)
    (:`Update`
      (`MaterialInstanceDynamic.SetScalarParameterValue` (stale `self.ReceiveBeginPlay` _returnvalue) "Hue" 0.5)
      (`MaterialInstanceDynamic.SetScalarParameterValue` (stale `self.ReceiveBeginPlay` _returnvalue) "Time" `_新建轨道_0`)
      (`KismetSystemLibrary.Delay` 0.5)
      (`self.K2_DestroyActor`))))

(fn `UserConstructionScript`)