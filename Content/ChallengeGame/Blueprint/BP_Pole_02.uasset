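; BP_Pole_02 is an animated challenge-game prop with two wooden poles moving vertically and four toothed gears turning.
; On BeginPlay it caches both pole positions, then a timeline raises one by its track value and the other by that value's absolute difference from 150.
; That timeline's updates chain into two more timelines that pitch the gears in pairs.
; ForwardOrReverse flips each pair's direction, keeping the two pairs' track values oppositely signed.
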(event `self.ReceiveBeginPlay`
  (bind (_pos_01_x _pos_01_y _pos_01_z) (`KismetMathLibrary.BreakVector` (`self.Pos_01`)))
  (bind (_pos_02_x _pos_02_y _pos_02_z) (`KismetMathLibrary.BreakVector` (`self.Pos_02`)))
  (`TimelineComponent.SetPlayRate` (`self.时间轴_0`) 3.0)
  (set `self.Pos_01` (`SceneComponent.K2_GetComponentLocation` (`self.SM_WoodenPole_07`)))
  (set `self.Pos_02` (`SceneComponent.K2_GetComponentLocation` (`self.SM_WoodenPole_06`)))
  (bind (_direction `_新建轨道_0`) (`Timeline|时间轴_0`)
    (:`Update`
      (`SceneComponent.K2_SetWorldLocation` (`self.SM_WoodenPole_07`) (`KismetMathLibrary.MakeVector` _pos_01_x _pos_01_y (+ _pos_01_z `_新建轨道_0`)) false false)
      (`SceneComponent.K2_SetWorldLocation` (`self.SM_WoodenPole_06`) (`KismetMathLibrary.MakeVector` _pos_02_x _pos_02_y (+ _pos_02_z (`KismetMathLibrary.Abs` (- `_新建轨道_0` 150.0)))) false false)
      (bind (_direction_2 `_新建轨道_0_2`) (`Timeline|时间轴`)
        (:`Update`
          (if (`self.Forward or Reverse`)
            (`SceneComponent.K2_SetRelativeRotation` (`self.SM_ToothedGear_03`) (`KismetMathLibrary.MakeRotator` 0.0 `_新建轨道_0_2`) false false)
            (`SceneComponent.K2_SetRelativeRotation` (`self.SM_ToothedGear_02`) (`KismetMathLibrary.MakeRotator` 0.0 `_新建轨道_0_2`) false false)
            (bind (_direction_3 `_新建轨道_0_3`) (`Timeline|时间轴_1` :!label _label)
              (:`Update`
                (if (`self.Forward or Reverse`)
                  (`SceneComponent.K2_SetRelativeRotation` (`self.SM_ToothedGear_04`) (`KismetMathLibrary.MakeRotator` 0.0 (* `_新建轨道_0_3` -1.0)) false false)
                  (`SceneComponent.K2_SetRelativeRotation` (`self.SM_ToothedGear_01`) (`KismetMathLibrary.MakeRotator` 0.0 (* `_新建轨道_0_3` -1.0)) false false)
                  (else
                    (`SceneComponent.K2_SetRelativeRotation` (`self.SM_ToothedGear_01`) (`KismetMathLibrary.MakeRotator` 0.0 `_新建轨道_0_3`) false false)
                    (`SceneComponent.K2_SetRelativeRotation` (`self.SM_ToothedGear_04`) (`KismetMathLibrary.MakeRotator` 0.0 `_新建轨道_0_3`) false false)))))
            (else
              (`SceneComponent.K2_SetRelativeRotation` (`self.SM_ToothedGear_02`) (`KismetMathLibrary.MakeRotator` 0.0 (* `_新建轨道_0_2` -1.0)) false false)
              (`SceneComponent.K2_SetRelativeRotation` (`self.SM_ToothedGear_03`) (`KismetMathLibrary.MakeRotator` 0.0 (* `_新建轨道_0_2` -1.0)) false false)
              (goto _label))))))))

(fn `UserConstructionScript`)